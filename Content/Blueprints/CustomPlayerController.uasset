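; Player controller that sets up Enhanced Input, a camera actor view and jumping for the player character.
; On BeginPlay it adds the gameplay mapping context and switches the view target to a CameraActor found in the level.
; The jump input makes the Character pawn, looked up through GetMyPlayerIndex with an empty MatchID, jump and prints a debug message.
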(event Input|EnhancedActionEvents|EnhancedInputActionIA_Jump
  (params (ActionValue :type Boolean) (ElapsedSeconds :type Float%20%28double-precision%29) (TriggeredSeconds :type Float%20%28double-precision%29) (InputAction :type Input%20Action%20Object%20Reference :default "/Game/Input/IA_Jump.IA_Jump"))
  (:Triggered
    (CallFunction|JumpAction)
    (Development|PrintString "Boing!")))

(event EventBeginPlay
  (CallFunction|SetInputMap "/Game/Input/IMC_Gameplay1.IMC_Gameplay1")
  (bind _returnvalue (Actor|GetActorOfClass "/Script/Engine.CameraActor"))
  (Game|Player|SetViewTargetwithBlend _returnvalue 0.0 "VTBlend_Linear" 0.0 false))

(event EventTick
  (params (DeltaSeconds :type Float%20%28single-precision%29)))

(fn ConstructionScript)

(fn SetInputMap
  (params (NewParam :type Input%20Mapping%20Context%20Object%20Reference))
  (Input|AddMappingContext (PlayerController|LocalPlayerSubsystems|GetEnhancedInputLocalPlayerSubsystem self) NewParam 0 "(bIgnoreAllPressedKeysUntilRelease=True,bForceImmediately=False)"))

(fn JumpAction
  (bind _playerindex (Class|TurnBasedBlueprintLibrary|GetMyPlayerIndex self))
  (bind _ascharacter (Utilities|Casting|CastToCharacter (Game|Player|GetPlayerPawn _playerindex)))
  (Character|Jump _ascharacter))