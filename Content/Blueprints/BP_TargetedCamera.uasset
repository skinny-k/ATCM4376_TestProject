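; BP_TargetedCamera is a spring-arm camera that follows the average location of a managed list of target actors, with input-scaled yaw rotation.
; Each Tick it eases toward that point, then lengthens the arm per target failing IsInFOV.
; When all pass, the arm also grows, but clamped.
; IsInFOV compares an angle from each target's own location and root forward vector to the camera's FOV, ignoring camera position.
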(event EventBeginPlay)

(event Collision|EventActorBeginOverlap
  (params (OtherActor :type Actor%20Object%20Reference)))

(event EventTick
  (params (DeltaSeconds :type Float%20%28single-precision%29))
  (bind _springarm (Variables|Default|GetSpringArm))
  (bind _springarm_2 (Variables|Default|GetSpringArm))
  (bind _returnvalue (Class|GameplayStatics|GetActorArrayAverageLocation (Variables|Default|GettargetActors)))
  (Transformation|SetActorLocation (Math|Interpolation|VInterpTo (Transformation|GetActorLocation) _returnvalue DeltaSeconds (Variables|Default|GetinterpolationSpeed)) false false)
  (for _array_element (Variables|Default|GettargetActors)
    (bind _isinfov (CallFunction|IsinFOV (Variables|Default|GetMainCamera) _array_element))
    (if (not _isinfov)
      (Variables|/Script/Engine.SpringArmComponent|SetTargetArmLength _springarm_2 (+ (Variables|/Script/Engine.SpringArmComponent|GetTargetArmLength _springarm_2) (* (Variables|Default|GetinterpolationSpeed) DeltaSeconds)))
      (Variables|Default|SetFOVTooSmall true)))
  (if (Variables|Default|GetFOVTooSmall)
    _
    (else
      (Variables|/Script/Engine.SpringArmComponent|SetTargetArmLength _springarm (Math|Float|Clamp(Float) (+ (Variables|/Script/Engine.SpringArmComponent|GetTargetArmLength _springarm) (* (Variables|Default|GetinterpolationSpeed) DeltaSeconds)) 3.4e+02 5e+03))))
  (Variables|Default|SetFOVTooSmall false))

(fn ConstructionScript)

(fn AddTargetActor
  (params (newTarget :type Actor%20Object%20Reference))
  (Utilities|Array|AddUnique (Variables|Default|GettargetActors) newTarget))

(fn RemoveTargetActor
  (params (removeTarget :type Actor%20Object%20Reference))
  (Utilities|Array|RemoveItem (Variables|Default|GettargetActors) removeTarget))

(fn RotateThisFrame
  (params (deltaSeconds :type Float%20%28double-precision%29) (input :type Float%20%28double-precision%29))
  (Class|Actor|AddActorWorldRotation (Math|Rotator|MakeRotator 0.0 0.0 (* (* (Variables|Default|GetrotationalSpeed) deltaSeconds) input))))

(fn IsinFOV
  (params (Camera :type Camera%20Component%20Object%20Reference) (ActorToCheck :type Actor%20Object%20Reference))
  (bind _returnvalue (Transformation|GetActorLocation ActorToCheck))
  (bind _rootcomponent (Variables|/Script/Engine.Actor|GetRootComponent ActorToCheck))
  (bind _returnvalue_2 (Transformation|GetWorldLocation _rootcomponent))
  (bind _returnvalue_3 (- _returnvalue _returnvalue_2))
  (bind _returnvalue_4 (Math|Vector|VectorLength _returnvalue_3))
  (return (<= (* 4.0 (Class|KismetMathLibrary|DegAsin (/ (/ (Math|Vector|VectorLength (- _returnvalue (+ (* (Math|Vector|GetForwardVector _rootcomponent) _returnvalue_4) _returnvalue_2))) 2.0) _returnvalue_4))) (Variables|/Script/Engine.CameraComponent|GetFieldOfView Camera))))