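; Test actor that registers itself as a target of the BP_TargetedCamera in the level.
; On BeginPlay it looks up the camera, spawning one at the world origin and retrying if none exists, then adds itself through AddTargetActor.
; Tick adds it again once, gated by an Activated flag that BeginPlay never sets, and does not check that the camera is valid.
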(event EventBeginPlay
  (bind _returnvalue (Actor|GetActorOfClass "/Game/Blueprints/BP_TargetedCamera.BP_TargetedCamera_C" :!label _label))
  (if (Utilities|IsValid _returnvalue)
    (Default|AddTargetActor _returnvalue self)
    (else
      (Game|SpawnActorfromClass "/Game/Blueprints/BP_TargetedCamera.BP_TargetedCamera_C" (Math|Transform|MakeTransform "0, 0, 0") "Undefined" "MultiplyWithRoot" 0 0)
      (goto _label))))

(event Collision|EventActorBeginOverlap
  (params (OtherActor :type Actor%20Object%20Reference)))

(event EventTick
  (params (DeltaSeconds :type Float%20%28single-precision%29))
  (if (not (Variables|Default|Getactivated))
    (bind _returnvalue (Actor|GetActorOfClass "/Game/Blueprints/BP_TargetedCamera.BP_TargetedCamera_C"))
    (Default|AddTargetActor _returnvalue self)
    (Variables|Default|Setactivated true)))

(fn ConstructionScript)