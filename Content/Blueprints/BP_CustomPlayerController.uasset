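; BP_CustomPlayerController is a player controller that adds an Enhanced Input mapping context and hooks the player into a targeted camera.
; On BeginPlay it applies its default input map, sets the level's BP_TargetedCamera as view target, and registers the controlled pawn as a camera target.
; When destroyed, it removes the controlled pawn from that camera's targets.
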(event EventBeginPlay
  (CallFunction|SetInputMap (Variables|Default|GetdefaultInputMap))
  (bind _returnvalue (Actor|GetActorOfClass "/Game/Blueprints/BP_TargetedCamera.BP_TargetedCamera_C"))
  (Game|Player|SetViewTargetwithBlend _returnvalue 0.0 "VTBlend_Linear" 0.0 false)
  (Default|AddTargetActor _returnvalue (Pawn|GetControlledPawn)))

(event EventTick
  (params (DeltaSeconds :type Float%20%28single-precision%29)))

(event EventDestroyed
  (bind _returnvalue (Actor|GetActorOfClass "/Game/Blueprints/BP_TargetedCamera.BP_TargetedCamera_C"))
  (Default|RemoveTargetActor _returnvalue (Pawn|GetControlledPawn)))

(fn ConstructionScript)

(fn SetInputMap
  (params (NewParam :type Input%20Mapping%20Context%20Object%20Reference))
  (Input|AddMappingContext (PlayerController|LocalPlayerSubsystems|GetEnhancedInputLocalPlayerSubsystem self) NewParam 0 "(bIgnoreAllPressedKeysUntilRelease=True,bForceImmediately=False)"))