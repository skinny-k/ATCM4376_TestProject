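; Player character for GameMode1, colored by player index, with move, jump, crouch and dash abilities.
; Enhanced Input feeds movement directly and hands actions to jump, crouch and dash components, with jump plus crouch within a short window triggering a dash.
; A looping timer copies the floor's physical material friction into CharacterMovement and picks braking deceleration by surface type, making ice slippery.
; Animation calls and surface-based speed are present but disconnected.
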(event Custom|SetGroundFriction
  (bind _data (Variables|Default|GetData))
  (bind _charactermovement (Variables|Character|GetCharacterMovement))
  (bind _currentfloor (Variables|/Script/Engine.CharacterMovementComponent|GetCurrentFloor _charactermovement))
  (bind _physmat (Collision|BreakHitResult (.hitresult _currentfloor)))
  (if (Utilities|IsValid _physmat)
    (Variables|/Script/Engine.CharacterMovementComponent|SetGroundFriction (Variables|Character|GetCharacterMovement) (Variables|/Script/PhysicsCore.PhysicalMaterial|GetFriction _physmat)))
  (Variables|/Script/Engine.CharacterMovementComponent|SetBrakingDecelerationWalking (Variables|Character|GetCharacterMovement) (Utilities|Select :Index (Collision|GetSurfaceType (.hitresult _currentfloor)) :SurfaceType_Default (Variables|/Game/GameMode1/Programming/Player/Systems/Data/PDA_Player_GM1.PDA_Player_GM1_C|GetBraking%20--%20Default _data) :SurfaceType1 (Variables|/Game/GameMode1/Programming/Player/Systems/Data/PDA_Player_GM1.PDA_Player_GM1_C|GetBraking%20--%20Slippery _data))))

(event EventBeginPlay
  (bind _index (Variables|Default|GetIndex))
  (bind _returnvalue (Utilities|Select :Index _index :Option%200 "/Game/GameMode1/Art/PlayerMaterials/MI_PlayerMat_Blue.MI_PlayerMat_Blue" :Option%201 "/Game/GameMode1/Art/PlayerMaterials/MI_PlayerMat_Green.MI_PlayerMat_Green" :Option%202 "/Game/GameMode1/Art/PlayerMaterials/MI_PlayerMat_Red.MI_PlayerMat_Red" :Option%203 "/Game/GameMode1/Art/PlayerMaterials/MI_PlayerMat_Yellow.MI_PlayerMat_Yellow"))
  ;[0 0 0 0.5] Color
  (Rendering|Material|SetMaterial (Variables|Default|GetCylinder) 0 _returnvalue)
  (Rendering|Material|SetMaterial (Variables|Character|GetMesh) 0 _returnvalue)
  (Utilities|Time|SetTimerbyFunctionName 0 "SetGroundFriction" 0.1 true))

(fn ConstructionScript)

(fn ApplyMovement
  (params (ActionValue :type Vector%202D%20Structure))
  (bind (_x _y) (Math|Vector2D|BreakVector2D ActionValue))
  ;[0 0 0 0.5] Horizontal Movement
  (Pawn|Input|AddMovementInput (Game|Player|GetPlayerPawn (Variables|Default|GetIndex)) (Utilities|GetHorizontalWorldDirection) _x false)
  ;[0 0 0 0.5] Vertical Movement
  (Pawn|Input|AddMovementInput (Game|Player|GetPlayerPawn (Variables|Default|GetIndex)) (Utilities|GetVerticalWorldDirection) _y false))

(fn ApplyRotation
  (params (ActionValue :type Vector%202D%20Structure))
  (bind (_x _y) (Math|Vector2D|BreakVector2D ActionValue))
  ;[0 0 0 0.5] Rotation
  (Pawn|SetControlRotation (Game|GetPlayerController (Variables|Default|GetIndex)) (Math|Rotator|MakeRotator 0.0 0.0 (Class|KismetMathLibrary|DegAtan2 _y _x))))

(fn HandleDash
  (params (JumpTriggeredSeconds :type Float%20%28double-precision%29) (CrouchTriggeredSeconds :type Float%20%28double-precision%29))
  (if (Math|Boolean|ANDBoolean (Input|EnhancedActionValues|GetIA_Jump_GM1) (Input|EnhancedActionValues|GetIA_Crouch_GM1) (and (<= JumpTriggeredSeconds 0.5) (<= CrouchTriggeredSeconds 0.5)))
    (Default|EndCrouch (Variables|Default|GetAC_Crouch))
    (Default|EndJump (Variables|Default|GetAC_Jump))
    (Default|TrytoDash (Variables|Default|GetAC_Dash))
    (else
      (Default|EndDash (Variables|Default|GetAC_Dash)))))

(fn HandleKill
  (Default|CallOnDie self))

(event Input|EnhancedActionEvents|EnhancedInputActionIA_Jump_GM1
  (params (ActionValue :type Boolean) (ElapsedSeconds :type Float%20%28double-precision%29) (TriggeredSeconds :type Float%20%28double-precision%29) (InputAction :type Input%20Action%20Object%20Reference :default "/Game/GameMode1/Programming/Player/Input/Actions/IA_Jump_GM1.IA_Jump_GM1"))
  (:Triggered
    (if (stale Input|EnhancedActionEvents|EnhancedInputActionIA_Crouch_GM1 ActionValue)
      (CallFunction|HandleDash TriggeredSeconds (stale Input|EnhancedActionEvents|EnhancedInputActionIA_Crouch_GM1 TriggeredSeconds))))
  (:Started
    (Utilities|FlowControl|DelayUntilNextTick)
    (Default|TrytoJump (Variables|Default|GetAC_Jump))))

(event Input|EnhancedActionEvents|EnhancedInputActionIA_Crouch_GM1
  (params (ActionValue :type Boolean) (ElapsedSeconds :type Float%20%28double-precision%29) (TriggeredSeconds :type Float%20%28double-precision%29) (InputAction :type Input%20Action%20Object%20Reference :default "/Game/GameMode1/Programming/Player/Input/Actions/IA_Crouch_GM1.IA_Crouch_GM1"))
  (:Triggered
    (if (stale Input|EnhancedActionEvents|EnhancedInputActionIA_Jump_GM1 ActionValue)
      (CallFunction|HandleDash (stale Input|EnhancedActionEvents|EnhancedInputActionIA_Jump_GM1 TriggeredSeconds) TriggeredSeconds)))
  (:Started
    (Utilities|FlowControl|DelayUntilNextTick)
    (Default|TrytoCrouch (Variables|Default|GetAC_Crouch)))
  (:Completed
    (Default|EndCrouch (Variables|Default|GetAC_Crouch))))

(event Input|EnhancedActionEvents|EnhancedInputActionIA_StartGame_GM1
  (params (ActionValue :type Boolean) (ElapsedSeconds :type Float%20%28double-precision%29) (TriggeredSeconds :type Float%20%28double-precision%29) (InputAction :type Input%20Action%20Object%20Reference :default "/Game/GameMode1/Programming/Player/Input/Actions/IA_StartGame_GM1.IA_StartGame_GM1"))
  (:Completed
    (Class|BIGM1|StartGame(Message) (Game|GetGameMode))))

(event Input|EnhancedActionEvents|EnhancedInputActionIA_Move_GM1
  (params (ActionValue :type Vector%202D%20Structure) (ElapsedSeconds :type Float%20%28double-precision%29) (TriggeredSeconds :type Float%20%28double-precision%29) (InputAction :type Input%20Action%20Object%20Reference :default "/Game/GameMode1/Programming/Player/Input/Actions/IA_Move_GM1.IA_Move_GM1"))
  ;[0 0 0 0.5] Move
  (:Triggered
    (CallFunction|ApplyMovement ActionValue)))

(event EventOnLanded
  (params (Hit :type Hit%20Result%20Structure%20%28by%20ref%29))
  ;[0 0 0 0.5] Move
  (Default|EndJump (Variables|Default|GetAC_Jump)))

(event EventTick
  (params (DeltaSeconds :type Float%20%28single-precision%29)))

(event Input|KeyboardEvents|Escape
  (params (Key :type Key%20Structure))
  (:Pressed
    (Game|QuitGame (Game|GetPlayerController (Variables|Default|GetIndex)) "Quit" false)))