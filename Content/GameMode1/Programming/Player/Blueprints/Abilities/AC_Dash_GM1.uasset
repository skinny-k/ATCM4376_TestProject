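; Dash ability component for the GameMode1 player that launches the character forward and shoves players in the way.
; TryToDash checks player state (jumping, crouched, already dashing), then StartDash launches, flags dashing and ends any jump, behind a DoOnce with no reset here.
; A short forward sphere trace then knocks back any player hit.
; The dashing flag clears only if that same pass finds velocity near zero or EndDash is called.
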(fn TrytoDash
  (bind _candash (CallFunction|CheckCanDash))
  (if _candash
    (CallFunction|StartDash)
    (CallFunction|CheckHitOtherPlayer)))

(fn CheckCanDash
  (bind _as_bp_player_gm1 (Variables|Default|GetAs%20BP%20Player%20GM1))
  (return (Math|Boolean|ANDBoolean (Variables|/Game/GameMode1/Programming/Player/Blueprints/BP_Player_GM1.BP_Player_GM1_C|GetcanDash _as_bp_player_gm1) (not (Variables|/Game/GameMode1/Programming/Player/Blueprints/BP_Player_GM1.BP_Player_GM1_C|GetisJumping _as_bp_player_gm1)) (not (Variables|/Script/Engine.Character|GetbIsCrouched _as_bp_player_gm1)) (not (Variables|/Game/GameMode1/Programming/Player/Blueprints/BP_Player_GM1.BP_Player_GM1_C|GetisDashing _as_bp_player_gm1)) (not (Character|IsJumpProvidingForce _as_bp_player_gm1)))))

(fn StartDash
  (bind _as_bp_player_gm1 (Variables|Default|GetAs%20BP%20Player%20GM1))
  (Utilities|FlowControl|DoOnce false
    (:Completed
      (Character|LaunchCharacter (Variables|Default|GetAs%20BP%20Player%20GM1) (* (Math|Vector|GetForwardVector (Transformation|GetActorRotation (Variables|Default|GetAs%20BP%20Player%20GM1))) 2e+03) true false)
      (Variables|/Game/GameMode1/Programming/Player/Blueprints/BP_Player_GM1.BP_Player_GM1_C|SetisDashing _as_bp_player_gm1 true)
      (Default|EndJump (Variables|/Game/GameMode1/Programming/Player/Blueprints/BP_Player_GM1.BP_Player_GM1_C|GetAC_Jump _as_bp_player_gm1)))))

(fn CheckHitOtherPlayer
  (bind _as_bp_player_gm1 (Variables|Default|GetAs%20BP%20Player%20GM1))
  (bind _as_bp_player_gm1_2 (Variables|Default|GetAs%20BP%20Player%20GM1))
  (bind _returnvalue (Transformation|GetActorLocation _as_bp_player_gm1))
  (bind _returnvalue_2 (Transformation|GetActorRotation _as_bp_player_gm1_2))
  (bind _returnvalue_3 (Math|Vector|GetForwardVector _returnvalue_2))
  (bind _returnvalue_4 (* _returnvalue_3 1e+03))
  (bind _outhit (Collision|SphereTraceForObjects _returnvalue (+ _returnvalue (* (Transformation|GetActorForwardVector _as_bp_player_gm1) 1e+02)) 1e+01 (Utilities|Array|MakeArray "ObjectTypeQuery3") false 0 "ForOneFrame"))
  (if (.bBlockingHit (Collision|BreakHitResult _outhit))
    (Character|LaunchCharacter (.AsBP%20Player%20GM1 (Utilities|Casting|CastToBP_Player_GM1 (.HitActor (Collision|BreakHitResult _outhit)))) (Math|Vector|MakeVector (.x _returnvalue_4) (.y _returnvalue_4) 0.0) true false))
  (CallFunction|CheckifEndDash))

(fn EndDash
  (Variables|/Game/GameMode1/Programming/Player/Blueprints/BP_Player_GM1.BP_Player_GM1_C|SetisDashing (Variables|Default|GetAs%20BP%20Player%20GM1) false))

(fn CheckifEndDash
  (if (<= (Math|Vector|VectorLength (Transformation|GetVelocity (Variables|Default|GetAs%20BP%20Player%20GM1))) 1.0)
    (CallFunction|EndDash)))